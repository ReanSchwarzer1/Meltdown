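; Crafting table actor that opens the crafting menu when a Doctor or Soldier character overlaps it.
; Overlap stores the character, then immediately locks player 0's look and move input, creates the menu widget, disables controller input and shows the cursor.
; An E press while overlapped runs the same path.
; Ending overlap clears references, hides menu and cursor, and restores look input only, leaving move input ignored and controller input disabled.
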(event EventBeginPlay)

(event Collision|EventActorBeginOverlap
  (params (OtherActor :type Actor%20Object%20Reference))
  (bind _returnvalue (Game|GetPlayerController 0))
  (bind _returnvalue_2 (Game|GetPlayerController 0))
  (bind _asbp_doctor (Utilities|Casting|CastToBP_Doctor OtherActor)
    (:then
      (Variables|Default|SetDoctor _asbp_doctor))
    (:CastFailed
      (bind _asbp_soldier (Utilities|Casting|CastToBP_Soldier OtherActor))
      (Variables|Default|SetSoldier _asbp_soldier)))
  (Variables|Default|SetisOverlapped true) ; Ideally this would not auto trigger on overlap, but for now it will
  (Utilities|FlowControl|Sequence
    (:then_0
      (Input|SetIgnoreLookInput _returnvalue_2 true)
      (Input|SetIgnoreMoveInput _returnvalue_2 true))
    (:then_1
      (Variables|Default|GetSoldier
        (:then
          _)
        (:else
          (Variables|Default|GetDoctor
            (:then
              _)
            (:else))))
      (bind _returnvalue_3 (UserInterface|CreateWidget "/Game/UI/Crafting_Menu/BP_Crafting_Menu.BP_Crafting_Menu_C" _returnvalue))
      (UserInterface|Viewport|AddtoViewport _returnvalue_3 0)
      (Input|DisableInput _returnvalue)
      (Variables|/Script/Engine.PlayerController|SetbShowMouseCursor (Game|GetPlayerController (Variables|/Script/Engine.Pawn|GetPlayerState (Game|Player|GetPlayerPawn 0))) true))))

(event EventTick
  (params (DeltaSeconds :type Float%20%28single-precision%29)))

(event Collision|EventActorEndOverlap
  (params (OtherActor :type Actor%20Object%20Reference))
  (Variables|Default|SetisOverlapped false)
  (Variables|Default|SetDoctor 0)
  (Variables|Default|SetSoldier 0)
  (Input|SetIgnoreLookInput (Game|GetPlayerController 0) false)
  (Widget|SetVisibility (stale Collision|EventActorBeginOverlap _returnvalue_3) "Hidden")
  (Variables|/Script/Engine.PlayerController|SetbShowMouseCursor (Game|GetPlayerController (Variables|/Script/Engine.Pawn|GetPlayerState (Game|Player|GetPlayerPawn 0))) false))

(event Input|KeyboardEvents|E
  (params (Key :type Key%20Structure :default "None"))
  (bind _returnvalue (Game|GetPlayerController 0))
  (bind _returnvalue_2 (Game|GetPlayerController 0))
  (:Pressed
    (if (Variables|Default|GetisOverlapped)
      (Utilities|FlowControl|Sequence
        (:then_0
          (Input|SetIgnoreLookInput _returnvalue_2 true)
          (Input|SetIgnoreMoveInput _returnvalue_2 true))
        (:then_1
          (Variables|Default|GetSoldier
            (:then
              _)
            (:else
              (Variables|Default|GetDoctor
                (:then
                  _)
                (:else))))
          (bind _returnvalue_3 (UserInterface|CreateWidget "/Game/UI/Crafting_Menu/BP_Crafting_Menu.BP_Crafting_Menu_C" _returnvalue))
          (UserInterface|Viewport|AddtoViewport _returnvalue_3 0)
          (Input|DisableInput _returnvalue)
          (Variables|/Script/Engine.PlayerController|SetbShowMouseCursor (Game|GetPlayerController (Variables|/Script/Engine.Pawn|GetPlayerState (Game|Player|GetPlayerPawn 0))) true))))))

(fn ConstructionScript)